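; Base patroller enemy that periodically damages pawns in front of it and carries a health widget.
; Damageable interface calls forward to BPC_DamageSystem, whose death and damage-response dispatchers are bound in the construction script.
; A looping timer runs a short forward sphere trace, with debug drawing, and sends damage to the hit actor.
; Death ragdolls the mesh before destroying the actor, while damage responses are only printed.
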(event `Death`
  (bind _mesh (`self.Mesh`))
  ;[1 1 1] Event Dispatchers Used In Construction Script Of This Class & BPC_DamageSystem
  (`KismetSystemLibrary.PrintString` "Dead")
  (`PrimitiveComponent.SetSimulatePhysics` _mesh true)
  (`PrimitiveComponent.SetCollisionEnabled` _mesh "QueryAndPhysics")
  (`KismetSystemLibrary.Delay` 1.0)
  (`self.K2_DestroyActor`))

(event `DamageResponse`
  (params (DamageResponse :type "/Game/Assignment/Mo/Damage_System/E_DamageResponse Enum" :default "NewEnumerator0"))
  ;[1 1 1] Event Dispatchers Used In Construction Script Of This Class & BPC_DamageSystem
  (`KismetSystemLibrary.PrintString` (`|GetEnumeratorNameAsString` DamageResponse)))

(event `self.ReceiveBeginPlay`
  (`|ExecutionSequence`
    (:`then_0`
      (bind _returnvalue (`|CreateWidget` "/Game/Assignment/Liv/ui/mm/Mo_HP_Widget.Mo_HP_Widget_C" null self))
      (`WidgetComponent.SetWidget` (`self.Widget`) _returnvalue))
    (:`then_1`
      (`KismetSystemLibrary.K2_SetTimerDelegate` (delegate `DamagePlayer`) 2.0 true))))

(event `DamagePlayer`
  (bind _returnvalue (`self.K2_GetActorLocation`))
  (bind (_outhit _returnvalue_2) (`KismetSystemLibrary.SphereTraceSingleForObjects` :`Start` _returnvalue :`End` (+ _returnvalue (* (`self.GetActorForwardVector`) 100.0)) :`Radius` 20.0 :`ObjectTypes` (`|MakeArray` "ObjectTypeQuery3" :!type "EObjectTypeQuery Enum") :`DrawDebugType` "ForDuration" :`TraceColor` (struct :`R` 1.0 :`B` 0.991945 :`A` 1.0) :`TraceHitColor` (struct :`G` 0.868705 :`B` 1.0 :`A` 1.0) :`DrawTime` 1.0))
  (if _returnvalue_2
    (message `/Game/Assignment/Mo/Damage_System/BPI_Damageable.TakeDamage` (`.HitActor` (`GameplayStatics.BreakHitResult` _outhit)) (make `/Game/Assignment/Mo/Damage_System/S_DamageInfo` 10.0 "NewEnumerator2" "NewEnumerator1"))))

(fn `GetCurrentHealth`
  (returns (Health :type "Float (double-precision)"))
  (return (`/Game/Assignment/Mo/Damage_System/BPC_DamageSystem.Health` (`self.BPC_DamageSystem`))))

(fn `GetMaxHealth`
  (returns (MaxHealth :type "Float (double-precision)"))
  (return (`/Game/Assignment/Mo/Damage_System/BPC_DamageSystem.MaxHealth` (`self.BPC_DamageSystem`))))

(fn `Heal`
  (params (Amount :type "Float (double-precision)"))
  (returns (NewHealth :type "Float (double-precision)"))
  (bind _newhealth (`/Game/Assignment/Mo/Damage_System/BPC_DamageSystem.Heal` (`self.BPC_DamageSystem`) Amount))
  (return _newhealth))

(fn `TakeDamage`
  (params (DamageInfo :type "/Game/Assignment/Mo/Damage_System/S_DamageInfo Structure"))
  (returns (`Was Damaged` :type Boolean))
  (bind _wasdamaged (`/Game/Assignment/Mo/Damage_System/BPC_DamageSystem.TakeDamage` (`self.BPC_DamageSystem`) DamageInfo))
  (return _wasdamaged))

(fn `UserConstructionScript`
  (bind _bpc_damagesystem (`self.BPC_DamageSystem`))
  (add `/Game/Assignment/Mo/Damage_System/BPC_DamageSystem.OnDeath` _bpc_damagesystem (`|CreateDelegate` :!event `Death`))
  (add `/Game/Assignment/Mo/Damage_System/BPC_DamageSystem.OnDamageResponse` _bpc_damagesystem (`|CreateDelegate` :!event `DamageResponse`)))